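; Game mode for an infinite runner that builds the track from chained tiles and keeps the score.
; On BeginPlay it populates a pool of nav mesh bounds volumes, then spawns the opening tiles.
; Each spawned tile receives the shared pool, and its attach location becomes the transform for the next tile.
; NewTileConqured adds a fixed reward to the score but spawns no tile itself.
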(event EventBeginPlay
  (Class|InfiniteTerrainGameMode|PopulateBoundsVolumePool)
  (for _index (range 0 3)
    (CallFunction|SpawnTile)))

(fn ConstructionScript)

(fn SpawnTile
  (bind _returnvalue (Game|SpawnActorfromClass "/Game/Dynamic/Terrain/Tile_BP.Tile_BP_C" (Variables|Default|GetNextTileTransform) "Undefined" 0 0))
  (Class|Tile|SetPool _returnvalue (Variables|Default|GetNavMeshBoundsVolumePool))
  (bind _attach_transform (Default|GetAttachLocation _returnvalue))
  (Variables|Default|SetNextTileTransform _attach_transform))

(fn NewTileConqured
  (Variables|Default|SetScore (+ (Variables|Default|GetScore) 100)))