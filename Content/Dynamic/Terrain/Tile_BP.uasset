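; An infinite runner terrain tile that, on spawn, locks its barrier and scatters random numbers of props and rocks via PlaceActors.
; The player entering LockingVolume unlocks the barrier, turning it green without collision; leaving relocks it red and asks InfiniteRunnerGameMode to spawn another tile.
; The player overlapping DestroyVolume destroys the tile.
; GetAttachLocation exposes the Arrow's world transform as an attach point.
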(event OnComponentBeginOverlap(LockingVolume)
  (params (OverlappedComponent :type Primitive%20Component%20Object%20Reference) (OtherActor :type Actor%20Object%20Reference) (OtherComp :type Primitive%20Component%20Object%20Reference) (OtherBodyIndex :type Integer) (bFromSweep :type Boolean) (SweepResult :type Hit%20Result%20Structure%20%28by%20ref%29))
  (Utilities|IsPlayerActor OtherActor)
  (CallFunction|Unlock))

(event OnComponentEndOverlap(LockingVolume)
  (params (OverlappedComponent :type Primitive%20Component%20Object%20Reference) (OtherActor :type Actor%20Object%20Reference) (OtherComp :type Primitive%20Component%20Object%20Reference) (OtherBodyIndex :type Integer))
  (Utilities|IsPlayerActor OtherActor)
  (CallFunction|Lock)
  (bind _asinfinite_runner_game_mode (Utilities|Casting|CastToInfiniteRunnerGameMode (Game|GetGameMode)))
  (Default|SpawnTile _asinfinite_runner_game_mode))

(event OnComponentBeginOverlap(DestroyVolume)
  (params (OverlappedComponent :type Primitive%20Component%20Object%20Reference) (OtherActor :type Actor%20Object%20Reference) (OtherComp :type Primitive%20Component%20Object%20Reference) (OtherBodyIndex :type Integer) (bFromSweep :type Boolean) (SweepResult :type Hit%20Result%20Structure%20%28by%20ref%29))
  (Utilities|IsPlayerActor OtherActor)
  (Actor|DestroyActor))

(event EventBeginPlay
  (CallFunction|Lock)
  (Class|Tile|PlaceActors "/Game/Dynamic/Terrain/Props/BP_Container.BP_Container_C" 1 3)
  (Class|Tile|PlaceActors "/Game/Dynamic/Terrain/Props/BP_Box.BP_Box_C" 2 4)
  (Class|Tile|PlaceActors "/Game/Dynamic/Terrain/Props/BP_Canister.BP_Canister_C" 1 7)
  (Class|Tile|PlaceActors "/Game/Dynamic/Terrain/Props/BP_Sack.BP_Sack_C" 1 3)
  (Class|Tile|PlaceActors "/Game/Dynamic/Terrain/Props/BP_Rock01_High.BP_Rock01_High_C" 0 5)
  (Class|Tile|PlaceActors "/Game/Dynamic/Terrain/Props/BP_Rock05_High.BP_Rock05_High_C" 0 5)
  (Class|Tile|PlaceActors "/Game/Dynamic/Terrain/Props/BP_Rock17_High.BP_Rock17_High_C" 0 5))

(fn ConstructionScript)

(fn GetAttachLocation
  (return (Transformation|GetWorldTransform (Variables|Default|GetArrow))))

(fn Unlock
  (Collision|SetCollisionEnabled (Variables|Default|GetBarrier) "NoCollision")
  (Rendering|Material|SetMaterial (Variables|Default|GetBarrier) 0 "/Game/Dynamic/Terrain/GreenBarrier.GreenBarrier"))

(fn Lock
  (Collision|SetCollisionEnabled (Variables|Default|GetBarrier) "QueryAndPhysics")
  (Rendering|Material|SetMaterial (Variables|Default|GetBarrier) 0 "/Game/Dynamic/Terrain/RedBarrier.RedBarrier"))